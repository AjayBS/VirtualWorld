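; Player character Blueprint with movement along world X, variable-height jumping, wall jumps and a counter-limited air jump.
; Pressing Jump while falling line-traces along the forward axis, from just behind the capsule to just in front.
; A hit launches the character up and away from the wall; otherwise it calls Jump if the counter allows, and landing resets the counter.
; The Construction Script sets jump velocity and hold time.
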(event `InputAxis|MoveRight`
  (params (AxisValue :type "Float (single-precision)"))
  ;[1 1 1] Movement
  (`self.AddMovementInput` (1.0 0.0 0.0) AxisValue))

(event `InputAction|Jump`
  (params (Key :type "Key Structure" :default "AnyKey"))
  ;[1 1 1] Jumping
  (:`Pressed`
    (set `CharacterMovementComponent.AirControl` 0.7 (`self.CharacterMovement`))
    (if (`NavMovementComponent.IsFalling` (`self.CharacterMovement`))
      (`self.WallJump`)
      (else
        (`self.Jump`)
        (set `self.NumberofJumps` (+ (`self.NumberofJumps`) 1)))))
  (:`Released`
    (`self.StopJumping`)))

(event `self.OnLanded`
  (params (Hit :type "HitResult Structure (by ref)"))
  ;[1 1 1] Landed
  (set `self.NumberofJumps` 0))

(event `WallJump`
  (bind _returnvalue (`self.GetActorForwardVector`))
  (bind _returnvalue_x (`KismetMathLibrary.BreakVector` (`self.K2_GetActorLocation`)))
  (bind (_outhit _returnvalue_2) (`KismetSystemLibrary.LineTraceSingle` (- (`self.K2_GetActorLocation`) (* _returnvalue (+ (`CapsuleComponent.GetScaledCapsuleRadius` (`self.CapsuleComponent`)) 15.0))) (+ (`self.K2_GetActorLocation`) (* _returnvalue (+ (`CapsuleComponent.GetScaledCapsuleRadius` (`self.CapsuleComponent`)) 15.0))) "TraceTypeQuery1" true))
  (if _returnvalue_2
    (`self.LaunchCharacter` (`KismetMathLibrary.MakeVector` (* (`KismetMathLibrary.SignOfFloat` (- _returnvalue_x (.x (`.Location` (`GameplayStatics.BreakHitResult` _outhit))))) 450.0) 0.0 (`CharacterMovementComponent.JumpZVelocity` (`self.CharacterMovement`))) true true)
    (elif (<= (`self.NumberofJumps`) 1)
      (`self.Jump`)
      (set `self.NumberofJumps` (+ (`self.NumberofJumps`) 1)))))

(fn `UserConstructionScript`
  (set `CharacterMovementComponent.JumpZVelocity` 400.0 (`self.CharacterMovement`))
  (set `self.JumpMaxHoldTime` 0.3)
  (set `self.NumberofJumps` 0))