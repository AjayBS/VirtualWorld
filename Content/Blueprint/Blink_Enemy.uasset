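; Enemy that blinks between two spots and ends the game when the player touches it.
; A looping three-second timer swaps its location between the BeginPlay position and a TargetPoint actor.
; Player overlap opens the GameOverMenu widget, disables input and shows the cursor.
; ToggleVisibility only teleports to the TargetPoint; timeline movement and visibility, collision and tick toggles are disconnected leftovers.
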(event `self.ReceiveActorBeginOverlap`
  (params (OtherActor :type "Actor Object Reference"))
  (bind _returnvalue (`GameplayStatics.GetPlayerController` 0))
  (if (== OtherActor (`GameplayStatics.GetPlayerCharacter` 0))
    (`KismetSystemLibrary.PrintString` (`KismetStringLibrary.Conv_BoolToString` (`self.Disabled?`)))
    (bind _returnvalue_2 (`|CreateWidget` "/Game/Menus/GameOverMenu.GameOverMenu_C"))
    (`UserWidget.AddToViewport` _returnvalue_2 0)
    (`self.DisableInput` (`GameplayStatics.GetPlayerCharacter` 0) _returnvalue)
    (set `PlayerController.bShowMouseCursor` true _returnvalue)))

(event `self.ReceiveBeginPlay`
  (set `self.StartPos` (`self.K2_GetActorLocation`))
  (`KismetSystemLibrary.K2_SetTimerDelegate` (delegate `Disappear_sprite`) 3.0 true))

(event `Disappear_sprite`
  (if (== (`self.K2_GetActorLocation`) (`self.StartPos`))
    (`self.K2_SetActorLocation` (`self.K2_GetActorLocation` (`self.TargetPoint`)))
    (else
      (`self.K2_SetActorLocation` (`self.StartPos`)))))

(fn `ToggleVisibility`
  (`self.K2_SetActorLocation` (`self.K2_GetActorLocation` (`self.TargetPoint`)) false true))

(fn `UserConstructionScript`)