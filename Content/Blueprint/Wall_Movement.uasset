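; Wall actor Blueprint that slides itself by a set offset when its Move_Wall event is called.
; The event stores the current location as StartPos and plays the Movement timeline from the start.
; Each update lerps the actor from StartPos to StartPos plus the Speed vector, which acts as a displacement, using the Move track as alpha, without sweep.
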(event `Move_Wall`
  (bind (_startpos_x _startpos_y _startpos_z) (`KismetMathLibrary.BreakVector` (`self.startPos`)))
  (bind (_speed_x _speed_y _speed_z) (`KismetMathLibrary.BreakVector` (`self.Speed`)))
  (set `self.startPos` (`self.K2_GetActorLocation`))
  (bind (_direction _move) (`Timeline|Movement` :!via `PlayFromStart`)
    (:`Update`
      (`self.K2_SetActorLocation` (`KismetMathLibrary.VLerp` (`self.startPos`) (`KismetMathLibrary.MakeVector` (+ _startpos_x _speed_x) (+ _startpos_y _speed_y) (+ _startpos_z _speed_z)) _move)))))

(event `self.ReceiveBeginPlay`)

(event `self.ReceiveTick`
  (params (DeltaSeconds :type "Float (single-precision)")))

(fn `UserConstructionScript`)